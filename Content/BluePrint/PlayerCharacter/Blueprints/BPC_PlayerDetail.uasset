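; Player component that tracks stamina, ammo and shield for BP_PlayerCharacter.
; On BeginPlay it derives each maximum from GameDifficulty, with higher difficulty values giving smaller pools.
; Increase functions cap at the maximum and clear an availability flag, while decrease functions return whether the resource could be spent, with stamina and ammo re-arming their flags.
; Each value change pushes straight to the character's HUD widget.
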(event `self.ReceiveBeginPlay`
  (bind _asbp_player_character (cast `/Game/BluePrint/PlayerCharacter/Blueprints/BP_PlayerCharacter` (`self.GetOwner`)))
  (set `self.Player Character BP` _asbp_player_character)
  (set `self.Max Stamina` (* (- 4 (`self.Game Difficulty`)) (`self.Max Stamina`)))
  (set `self.Max Ammo` (- 4 (`self.Game Difficulty`)))
  (set `self.Max Shield` (* (- 4 (`self.Game Difficulty`)) (`self.Max Shield`))))

(fn `Decrease Ammo`
  (returns (`Can Fire` :type Boolean))
  (set `self.Ammo Increase Available?` true)
  (if (< (`self.Current Ammo`) 1)
    (return false)
    (else
      (bind _result (`/Engine/EditorBlueprintResources/StandardMacros.DecrementInt` (`self.Current Ammo`))
        (:`  `
          (bind _output_get (set `self.Current Ammo` _result))
          (`/Game/UI/CharacterHud/WBP_MainHud.UpdateAmmunition` (`/Game/BluePrint/PlayerCharacter/Blueprints/BP_PlayerCharacter.Hud Widget` (`self.Player Character BP`)) _output_get)
          (return true))))))

(fn `Decrease Shield`
  (returns (`Can Shield?` :type Boolean))
  (if (not (== (`self.Current Shield`) 0.0))
    (bind _output_get (set `self.Current Shield` (- (`self.Current Shield`) (`self.Shield Drain`))))
    (`/Game/UI/CharacterHud/WBP_MainHud.UpdateShield` (`/Game/BluePrint/PlayerCharacter/Blueprints/BP_PlayerCharacter.Hud Widget` (`self.Player Character BP`)) _output_get (`self.Max Shield`))
    (return true)
    (else
      (return false))))

(fn `Decrease Stamina`
  (returns (`Can Sprint?` :type Boolean))
  (set `self.Stamina Increase Available?` true)
  (if (not (== (`self.Current Stamina`) 0.0))
    (set `self.Current Stamina` (- (`self.Current Stamina`) (`self.Stamina Cost`)))
    (`/Game/UI/CharacterHud/WBP_MainHud.UpdateStamina` (`/Game/BluePrint/PlayerCharacter/Blueprints/BP_PlayerCharacter.Hud Widget` (`self.Player Character BP`)) (`self.Current Stamina`) (`self.Max Stamina`))
    (return true)
    (else
      (return false))))

(fn `Increase Ammo`
  (if (< (`self.Current Ammo`) (`self.Max Ammo`))
    (bind _result (`/Engine/EditorBlueprintResources/StandardMacros.IncrementInt` (`self.Current Ammo`))
      (:`  `
        (bind _output_get (set `self.Current Ammo` _result))
        (`/Game/UI/CharacterHud/WBP_MainHud.UpdateAmmunition` (`/Game/BluePrint/PlayerCharacter/Blueprints/BP_PlayerCharacter.Hud Widget` (`self.Player Character BP`)) _output_get)
        (if (== (`self.Current Ammo`) (`self.Max Ammo`))
          (set `self.Ammo Increase Available?` false))))))

(fn `Increase Shield`
  (params (`Shield Increase` :type "Float (double-precision)"))
  (bind _returnvalue (+ `Shield Increase` (`self.Current Shield`)))
  (if (not (== (`self.Max Shield`) (`self.Current Shield`)))
    (if (>= _returnvalue (`self.Max Shield`))
      (set `self.Shield Increase Available` false)
      (set `self.Current Shield` (`self.Max Shield`))
      (else
        (set `self.Current Shield` _returnvalue)))
    (`/Game/UI/CharacterHud/WBP_MainHud.UpdateShield` (`/Game/BluePrint/PlayerCharacter/Blueprints/BP_PlayerCharacter.Hud Widget` (`self.Player Character BP`)) (`self.Current Shield`) (`self.Max Shield`))))

(fn `Increase Stamina`
  (params (`Stamina Increase` :type "Float (double-precision)"))
  (bind _returnvalue (+ `Stamina Increase` (`self.Current Stamina`)))
  (if (not (== (`self.Current Stamina`) (`self.Max Stamina`)))
    (if (>= _returnvalue (`self.Max Stamina`))
      (set `self.Stamina Increase Available?` false)
      (set `self.Current Stamina` (`self.Max Stamina`))
      (else
        (set `self.Current Stamina` _returnvalue)))
    (`/Game/UI/CharacterHud/WBP_MainHud.UpdateStamina` (`/Game/BluePrint/PlayerCharacter/Blueprints/BP_PlayerCharacter.Hud Widget` (`self.Player Character BP`)) (`self.Current Stamina`) (`self.Max Stamina`))))