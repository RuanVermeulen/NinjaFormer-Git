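; Falling barrel platform that flashes as a warning, then drops after the player touches it.
; BeginPlay caches the mesh's original material.
; The first Player-tagged overlap on the collision box starts a latent loop that alternates flash and original materials, then enables gravity and physics simulation on the main mesh.
; A setter function lets the flash material be swapped, and nothing in the file resets the platform after it falls.
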(event `self.ReceiveBeginPlay`
  (set `self.OrignionalMaterial` (`PrimitiveComponent.GetMaterial` (`self.MainMesh`) 0)))

(event `self.CollitionBox.OnComponentBeginOverlap`
  (params (OverlappedComponent :type "PrimitiveComponent Object Reference") (OtherActor :type "Actor Object Reference") (OtherComp :type "PrimitiveComponent Object Reference") (OtherBodyIndex :type Integer) (bFromSweep :type Boolean) (SweepResult :type "HitResult Structure (by ref)"))
  (if (and (`self.ActorHasTag` OtherActor "Player") (not (`self.Falling?`)))
    (set `self.Falling?` true)
    (set `self.CurrentCount` 0)
    (if (<= (`self.CurrentCount`) (`self.FlashCount`)) :!label _label
      (`PrimitiveComponent.SetMaterial` (`self.MainMesh`) 0 (`self.Material_Flash`))
      (`KismetSystemLibrary.Delay` 0.4)
      (`PrimitiveComponent.SetMaterial` (`self.MainMesh`) 0 (`self.OrignionalMaterial`))
      (`KismetSystemLibrary.Delay` 0.4)
      (`/Engine/EditorBlueprintResources/StandardMacros.IncrementInt` (`self.CurrentCount`)
        (:`  `
          (goto _label)))
      (else
        (`PrimitiveComponent.SetEnableGravity` (`self.MainMesh`) true)
        (`PrimitiveComponent.SetSimulatePhysics` (`self.MainMesh`) true)))))

(fn `SetFlashMaterial`
  (params (MaterialFlash :type "MaterialInterface Object Reference"))
  (set `self.Material_Flash` MaterialFlash))

(fn `UserConstructionScript`)