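; Enemy ranged projectile Blueprint that builds on a parent projectile class and can be blocked by shields.
; On BeginPlay it sets its shot delay before running the parent logic.
; Overlapping an actor tagged Shield destroys the projectile without calling the parent overlap handler, while any other overlap passes through to the parent.
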(event `self.ReceiveBeginPlay`
  (set `self.ShotDelay` 1.5)
  (`parent.ReceiveBeginPlay`))

(event `self.ReceiveActorBeginOverlap`
  (params (OtherActor :type "Actor Object Reference"))
  (if (`self.ActorHasTag` OtherActor "Shield")
    (`self.K2_DestroyActor`)
    (else
      (`parent.ReceiveActorBeginOverlap` OtherActor))))

(fn `UserConstructionScript`
  (`parent.UserConstructionScript`))