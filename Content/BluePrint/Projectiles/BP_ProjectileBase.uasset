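; BP_ProjectileBase is a base projectile Blueprint that damages tagged targets on overlap and has a short lifetime.
; Tick locks the ImpactSphere to its starting Y coordinate, constraining it to the XZ plane, and a DoOnce there starts a delayed self-destruct.
; Overlaps ignore PowerUp and Projectile actors; others destroy it, with damage applied only to those tagged "Vunerable".
; An Aligned flag is set shortly after BeginPlay but not read here.
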(event `self.ReceiveBeginPlay`
  (bind (_returnvalue_x _returnvalue_y) (`KismetMathLibrary.BreakVector` (`SceneComponent.K2_GetComponentLocation` (`self.ImpactSphere`))))
  (set `self.Starting Y Cordinate` _returnvalue_y)
  (`KismetSystemLibrary.Delay` 1.0)
  (set `self.Aligned?` true))

(event `self.ReceiveTick`
  (params (DeltaSeconds :type "Float (single-precision)"))
  (bind _impactsphere (`self.ImpactSphere`))
  (bind (_returnvalue_x _returnvalue_y _returnvalue_z) (`KismetMathLibrary.BreakVector` (`SceneComponent.K2_GetComponentLocation` _impactsphere)))
  (`SceneComponent.K2_SetWorldLocation` _impactsphere (`KismetMathLibrary.MakeVector` _returnvalue_x (`self.Starting Y Cordinate`) _returnvalue_z) false false)
  (`/Engine/EditorBlueprintResources/StandardMacros.DoOnce` false
    (:`Completed`
      (`KismetSystemLibrary.Delay` 2.0)
      (`self.K2_DestroyActor`))))

(event `self.ReceiveActorBeginOverlap`
  (params (OtherActor :type "Actor Object Reference"))
  (if (and (not (`self.ActorHasTag` OtherActor "PowerUp")) (not (`self.ActorHasTag` OtherActor "Projectile")))
    (if (`self.ActorHasTag` OtherActor "Vunerable")
      (`GameplayStatics.ApplyDamage` OtherActor 100.0))
    (`self.K2_DestroyActor`)))

(fn `UserConstructionScript`)