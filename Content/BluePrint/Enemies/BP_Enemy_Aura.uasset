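; BP_Enemy_Aura is an enemy Blueprint that deals contact-style damage continuously while it is alive.
; Each Tick calls the parent, then runs LineTraceForDamage if Alive is set.
; Despite its name, that function does a short Visibility sphere trace from the AttackDamagePosision component, offset using its rotation.
; Any hit actor takes heavy damage, with no cooldown or filter in this graph, so damage can repeat every frame.
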(event `self.ReceiveTick`
  (params (DeltaSeconds :type "Float (single-precision)"))
  (`parent.ReceiveTick` DeltaSeconds)
  (if (`self.Alive?`)
    (`self.LineTraceForDamage`)))

(fn `LineTraceForDamage`
  (bind _attack_damage_posision (`self.Attack Damage Posision`))
  (bind _returnvalue (`SceneComponent.K2_GetComponentLocation` _attack_damage_posision))
  (bind (_outhit _returnvalue_2) (`KismetSystemLibrary.SphereTraceSingle` :`Start` _returnvalue :`End` (+ _returnvalue (* (`SceneComponent.K2_GetComponentRotation` _attack_damage_posision) 25.0)) :`Radius` 20.0 :`TraceChannel` "TraceTypeQuery1" :`DrawTime` 1.0))
  (if _returnvalue_2
    (`GameplayStatics.ApplyDamage` (`.HitActor` (`GameplayStatics.BreakHitResult` _outhit)) 100.0)))

(fn `UserConstructionScript`
  (`parent.UserConstructionScript`))