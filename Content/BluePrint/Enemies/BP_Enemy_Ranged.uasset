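; Ranged enemy Blueprint that shoots projectiles at pawns tagged Player seen by its PlayerSensor.
; While alive, each sighting sets Firing and turns the enemy toward the player at its own height.
; If it can attack, it spawns BP_Projectile_EnemyRanged at AttackDamagePosision, then waits out a cooldown before clearing Firing.
; LineTraceForDamage offers short-range sphere-trace damage but is not called in this graph.
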(event `self.ReceiveTick`
  (params (DeltaSeconds :type "Float (single-precision)"))
  (`parent.ReceiveTick` DeltaSeconds))

(event `self.PlayerSensor.OnSeePawn`
  (params (Pawn :type "Pawn Object Reference"))
  (bind (_returnvalue_x _returnvalue_y) (`KismetMathLibrary.BreakVector` (`self.K2_GetActorLocation` Pawn)))
  (bind _returnvalue (`KismetMathLibrary.Conv_VectorToTransform` (`self.K2_GetActorLocation`)))
  ;[0.05098 0.05098 0.05098] Fire Projectile
  (if (`self.Alive?`)
    (if (`self.ActorHasTag` Pawn "Player")
      (set `self.Firing?` true)
      (`self.K2_SetActorRotation` (`KismetMathLibrary.FindRelativeLookAtRotation` (`KismetMathLibrary.MakeTransform` (`KismetMathLibrary.MakeVector` (.x (.location _returnvalue)) (.y (.location _returnvalue)) (.z (.location _returnvalue))) (`KismetMathLibrary.MakeRotator` (.roll (.rotation _returnvalue)) (.pitch (.rotation _returnvalue)) (.yaw (.rotation _returnvalue))) (.scale _returnvalue)) (`KismetMathLibrary.MakeVector` _returnvalue_x _returnvalue_y (.z (.location _returnvalue)))))
      (if (`self.CanAttack?`)
        (`|SpawnActorFromClass` "/Game/BluePrint/Projectiles/BP_Projectile_EnemyRanged.BP_Projectile_EnemyRanged_C" (`SceneComponent.K2_GetComponentToWorld` (`self.Attack Damage Posision`)) "Undefined" "MultiplyWithRoot" null null)
        (set `self.CanAttack?` false)
        (`KismetSystemLibrary.Delay` 3.0)
        (set `self.Firing?` false)
        (set `self.CanAttack?` true)))))

(fn `LineTraceForDamage`
  (bind _attack_damage_posision (`self.Attack Damage Posision`))
  (bind _returnvalue (`SceneComponent.K2_GetComponentLocation` _attack_damage_posision))
  (bind (_outhit _returnvalue_2) (`KismetSystemLibrary.SphereTraceSingle` :`Start` _returnvalue :`End` (+ _returnvalue (* (`SceneComponent.K2_GetComponentRotation` _attack_damage_posision) 25.0)) :`Radius` 20.0 :`TraceChannel` "TraceTypeQuery1" :`DrawTime` 1.0))
  (if _returnvalue_2
    (`GameplayStatics.ApplyDamage` (`.HitActor` (`GameplayStatics.BreakHitResult` _outhit)) 100.0)))

(fn `NewFunction`)

(fn `UserConstructionScript`
  (`parent.UserConstructionScript`))