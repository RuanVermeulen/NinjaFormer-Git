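; Base enemy character that patrols by walking forward and turning around at ledges and walls.
; Each tick while alive, sphere traces from an arrow component check for floor and non-Player obstacles; a DoOnce, reset when the path is clear, limits each blockage to one 180-degree turn.
; Overlap with a Projectile-tagged actor kills it, enabling mesh ragdoll physics, disabling movement and ignoring Pawn and Camera collision.
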(event `self.ReceiveTick`
  (params (DeltaSeconds :type "Float (single-precision)"))
  (bind _charactermovement (`self.CharacterMovement`))
  (if (`self.Alive?`)
    (`|ExecutionSequence`
      (:`then_0`
        (bind _floordetected (`self.LineTraceForFloor`))
        (if _floordetected
          (goto _label :!via `Reset`)
          (else
            (`/Engine/EditorBlueprintResources/StandardMacros.DoOnce` false :!label _label
              (:`Completed`
                (`/Engine/EditorBlueprintResources/StandardMacros.FlipFlop`
                  (:`A`
                    (`MovementComponent.StopMovementImmediately` _charactermovement)
                    (`self.K2_AddActorWorldRotation` (struct :`Yaw` 180.0)))
                  (:`B`
                    (`NavMovementComponent.StopActiveMovement` _charactermovement)
                    (`self.K2_AddActorWorldRotation` (struct :`Yaw` 180.0)))))))))
      (:`then_1`
        (`self.MoveForward`)))))

(event `MoveForward`
  (bind (_returnvalue_x _returnvalue_y) (`KismetMathLibrary.BreakVector` (`self.GetActorForwardVector`)))
  (`self.AddMovementInput` (`KismetMathLibrary.MakeVector` _returnvalue_x _returnvalue_y 1110.0)))

(event `self.CapsuleComponent.OnComponentBeginOverlap`
  (params (OverlappedComponent :type "PrimitiveComponent Object Reference") (OtherActor :type "Actor Object Reference") (OtherComp :type "PrimitiveComponent Object Reference") (OtherBodyIndex :type Integer) (bFromSweep :type Boolean) (SweepResult :type "HitResult Structure (by ref)"))
  (bind _capsulecomponent (`self.CapsuleComponent`))
  (if (`self.ActorHasTag` OtherActor "Projectile")
    (`PrimitiveComponent.SetSimulatePhysics` (`self.Mesh`) true)
    (`CharacterMovementComponent.DisableMovement` (`self.CharacterMovement`))
    (`PrimitiveComponent.SetCollisionResponseToChannel` _capsulecomponent "ECC_Pawn" "ECR_Ignore")
    (`PrimitiveComponent.SetCollisionResponseToChannel` _capsulecomponent "ECC_Camera" "ECR_Ignore")
    (`PrimitiveComponent.SetCollisionResponseToChannel` (`self.Mesh`) "ECC_Camera" "ECR_Ignore")
    (set `self.Alive?` false)))

(fn `LineTraceForFloor`
  (returns (FloorDetected :type Boolean))
  (bind _returnvalue (`SceneComponent.K2_GetComponentLocation` (`self.LineTrceFloorArrow`)))
  (bind (_outhit _returnvalue_2) (`KismetSystemLibrary.SphereTraceSingle` _returnvalue (+ _returnvalue (* (`self.GetActorUpVector`) -100.0)) 15.0 "TraceTypeQuery1"))
  (bind _walldetected (`self.LineTraceForWall`))
  (return (and (not _walldetected) _returnvalue_2)))

(fn `LineTraceForWall`
  (returns (WallDetected :type Boolean))
  (bind _returnvalue (`SceneComponent.K2_GetComponentLocation` (`self.LineTrceFloorArrow`)))
  (bind (_outhit _returnvalue_2) (`KismetSystemLibrary.SphereTraceSingle` _returnvalue (+ _returnvalue (* (`KismetMathLibrary.GetForwardVector` (`self.K2_GetActorRotation`)) 50.0)) 15.0 "TraceTypeQuery1"))
  (if (not _returnvalue_2)
    (return _returnvalue_2)
    (else
      (return (and (not (`self.ActorHasTag` (`.HitActor` (`GameplayStatics.BreakHitResult` _outhit)) "Player")) _returnvalue_2)))))

(fn `UserConstructionScript`)