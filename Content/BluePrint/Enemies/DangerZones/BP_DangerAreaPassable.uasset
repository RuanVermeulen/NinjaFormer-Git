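; BP_DangerAreaPassable is a danger zone that hurts overlapping actors and disappears once the player reaches its pass box.
; Overlapping the Collition component applies BaseDamage with the DT_ImutableDamage type, then destroys the other actor unless it has the Player tag.
; A separate PassBox component destroys the zone itself when a Player-tagged actor overlaps it.
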(event `self.Collition.OnComponentBeginOverlap`
  (params (OverlappedComponent :type "PrimitiveComponent Object Reference") (OtherActor :type "Actor Object Reference") (OtherComp :type "PrimitiveComponent Object Reference") (OtherBodyIndex :type Integer) (bFromSweep :type Boolean) (SweepResult :type "HitResult Structure (by ref)"))
  (`GameplayStatics.ApplyDamage` OtherActor (`self.Base Damage`) null self "/Game/BluePrint/Enemies/DangerZones/DT_ImutableDamage.DT_ImutableDamage_C")
  (if (not (`self.ActorHasTag` OtherActor "Player"))
    (`self.K2_DestroyActor` OtherActor)))

(event `self.PassBox.OnComponentBeginOverlap`
  (params (OverlappedComponent :type "PrimitiveComponent Object Reference") (OtherActor :type "Actor Object Reference") (OtherComp :type "PrimitiveComponent Object Reference") (OtherBodyIndex :type Integer) (bFromSweep :type Boolean) (SweepResult :type "HitResult Structure (by ref)"))
  (if (`self.ActorHasTag` OtherActor "Player")
    (`self.K2_DestroyActor`)))

(fn `UserConstructionScript`)